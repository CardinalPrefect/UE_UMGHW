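; BP_Player is the player pawn for GeometryCatcher, providing sideways movement and a pause toggle.
; The MoveRight axis adds movement input along the actor's right vector scaled by MaxSpeed, which Tick consumes as a swept, frame-rate-independent local offset.
; BeginPlay adds a BP_Pause widget to the viewport, and the P key toggles both its visibility and the game's paused state.
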(event `self.ReceiveBeginPlay`
  (bind _returnvalue (`|CreateWidget` "/Game/GeometryCatcher/Blueprints/BP_Pause.BP_Pause_C" (`GameplayStatics.GetPlayerController` 0)))
  (`UserWidget.AddToViewport` _returnvalue 0)
  (set `self.PauseWidget` _returnvalue))

(event `self.ReceiveTick`
  (params (DeltaSeconds :type "Float (single-precision)"))
  (bind _returnvalue (`self.ConsumeMovementInputVector`))
  (`self.K2_AddActorLocalOffset` (* _returnvalue DeltaSeconds) true))

(event `InputAxis|MoveRight`
  (params (AxisValue :type "Float (single-precision)"))
  (`self.AddMovementInput` (`self.GetActorRightVector`) (* AxisValue (`self.MaxSpeed`))))

(event `Key|P` :paused true
  (params (Key :type "Key Structure"))
  (bind _pausewidget (`self.PauseWidget`))
  (bind _returnvalue (not (`GameplayStatics.IsGamePaused`)))
  (:`Pressed`
    (if _returnvalue
      (`Widget.SetVisibility` _pausewidget "Visible")
      (else
        (`Widget.SetVisibility` _pausewidget "Hidden")))
    (`GameplayStatics.SetGamePaused` _returnvalue)))

(fn `UserConstructionScript`)